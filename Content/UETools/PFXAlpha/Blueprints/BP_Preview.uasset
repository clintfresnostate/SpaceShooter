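; BP_Preview is a display actor that lays out a grid of static meshes to preview the entries of its Materials array.
; The construction script builds five rows of 80 yawed meshes, stepping height along each row, and stores them in Meshes.
; Material lookup uses a row stride of 20, so successive rows overlap in the array.
; BeginPlay is empty; the MoveComponentTo animations and alternative grid builder are disconnected.
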(event EventBeginPlay)

(fn ConstructionScript
  (Utilities|Array|Clear (Variables|Default|GetMeshes))
  (Variables|Default|SetZ 0.0)
  (Variables|Default|SetRow 0)
  (Variables|Default|SetColumn 0)
  (for _index (range 0 4)
    (for _index_2 (range 0 79)
      (bind _returnvalue (AddComponent|AddStaticMeshComponent false (Math|Transform|MakeTransform (* (Math|Vector|MakeVector (Math|Conversions|ToFloat(Integer) (Variables|Default|GetColumn)) (Math|Conversions|ToFloat(Integer) (Variables|Default|GetRow)) (Variables|Default|GetZ)) "384.000000,384.000000,384.000000") "-45.000000,0.000000,0.000000")))
      (Rendering|Material|SetMaterial _returnvalue 0 (Utilities|Array|Get(acopy) (Variables|Default|GetMaterials) (+ (* (Variables|Default|GetRow) 20) (Variables|Default|GetColumn))))
      (Utilities|Array|Add (Variables|Default|GetMeshes) _returnvalue)
      (Variables|Default|SetColumn (+ (Variables|Default|GetColumn) 1))
      (Variables|Default|SetZ (+ (Variables|Default|GetZ) 0.5)))
    (Variables|Default|SetRow (+ (Variables|Default|GetRow) 1))
    (Variables|Default|SetColumn 0)
    (Variables|Default|SetZ 0.0)))